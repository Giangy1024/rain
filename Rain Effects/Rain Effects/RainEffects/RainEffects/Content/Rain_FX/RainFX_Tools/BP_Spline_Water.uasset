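; Rain FX tool actor that runs a water particle effect fed by a spline, configurable per instance.
; The construction script passes the Spline and spawn, trail, size range and speed settings to the SplineParticle component's user variables.
; A Type enum selects one of four material pairs for the effect, and each branch also applies UpFade.
; All setup happens at construction, with no active runtime event logic.
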(event EventBeginPlay)

(event Collision|EventActorBeginOverlap
  (params (OtherActor :type Actor%20Object%20Reference)))

(event EventTick
  (params (DeltaSeconds :type Float%20%28single-precision%29)))

(fn ConstructionScript
  (bind _spline_particle (Variables|Default|GetSpline_Particle))
  (bind _min_max_size_ (Variables|Default|GetMin/Max%28Size%29))
  (bind _type (Variables|Default|GetType))
  (bind _spline_particle_2 (Variables|Default|GetSpline_Particle))
  (bind _spline_particle_3 (Variables|Default|GetSpline_Particle))
  (bind (_x _y) (Math|Vector2D|BreakVector2D _min_max_size_))
  (Class|NiagaraComponent|SetVariableObject _spline_particle "spline" (Variables|Default|GetSpline))
  (Class|NiagaraComponent|SetVariableInt _spline_particle "spawn" (Variables|Default|GetSpawn_Count))
  (Class|NiagaraComponent|SetVariableInt _spline_particle "trail" (Variables|Default|GetTrail_Length))
  (Niagara|SetNiagaraVariable(Float) _spline_particle "scmin" _x)
  (Niagara|SetNiagaraVariable(Float) _spline_particle "scmax" _y)
  (Niagara|SetNiagaraVariable(Float) (Variables|Default|GetSpline_Particle) "speed" (Variables|Default|GetSpeed))
  (Utilities|FlowControl|Sequence
    (:then_0
      (if (Utilities|Enum|Equal(Enum) _type "NewEnumerator0")
        (Class|NiagaraComponent|SetVariableMaterial _spline_particle_3 "Mat" "/Game/Rain_FX/RainFX_Tools/Material/Master/M_SW_s_A.M_SW_s_A")
        (Class|NiagaraComponent|SetVariableMaterial _spline_particle_3 "Mat2" "/Game/Rain_FX/RainFX_Tools/Material/Master/M_SW_m_A.M_SW_m_A")
        (Niagara|SetNiagaraVariable(Float) _spline_particle_3 "UpFade" (Variables|Default|GetUp_Fade) :!label _label)))
    (:then_1
      (if (Utilities|Enum|Equal(Enum) _type "NewEnumerator1")
        (Class|NiagaraComponent|SetVariableMaterial _spline_particle_3 "Mat" "/Game/Rain_FX/RainFX_Tools/Material/Master/M_SW_s_B.M_SW_s_B")
        (Class|NiagaraComponent|SetVariableMaterial _spline_particle_3 "Mat2" "/Game/Rain_FX/RainFX_Tools/Material/Master/M_SW_m_B.M_SW_m_B")
        (goto _label)))
    (:then_2
      (if (Utilities|Enum|Equal(Enum) _type "NewEnumerator2")
        (Class|NiagaraComponent|SetVariableMaterial _spline_particle_2 "Mat" "/Game/Rain_FX/RainFX_Tools/Material/Master/M_SW_s_C.M_SW_s_C")
        (Class|NiagaraComponent|SetVariableMaterial _spline_particle_2 "Mat2" "/Game/Rain_FX/RainFX_Tools/Material/Master/M_SW_m_C.M_SW_m_C")
        (goto _label)))
    (:then_3
      (if (Utilities|Enum|Equal(Enum) _type "NewEnumerator3")
        (Class|NiagaraComponent|SetVariableMaterial _spline_particle_2 "Mat" "/Game/Rain_FX/RainFX_Tools/Material/Master/M_SW_s_D.M_SW_s_D")
        (Class|NiagaraComponent|SetVariableMaterial _spline_particle_2 "Mat2" "/Game/Rain_FX/RainFX_Tools/Material/Master/M_SW_m_D.M_SW_m_D")
        (goto _label)))))